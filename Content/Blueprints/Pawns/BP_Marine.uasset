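; BP_Marine is a player-controlled marine pawn that handles movement and horizontal aiming.
; Movement axis inputs drive it along its own forward and right vectors.
; Every tick, UpdatePlayerAim adds the right/left aim axis, scaled by RotationSpeed and delta time, to the character's yaw and sets it as control rotation.
; Aiming targets player index 0's controller and character rather than self, keeping pitch and roll from the actor.
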(event EventTick
  (params (DeltaSeconds :type Float%20%28single-precision%29))
  (CallFunction|UpdatePlayerAim))

(event Input|AxisEvents|InputAxisMoveForward/Backward
  (params (AxisValue :type Float%20%28single-precision%29))
  (Pawn|Input|AddMovementInput (Transformation|GetActorForwardVector) AxisValue false))

(event Input|AxisEvents|InputAxisMoveRight/Left
  (params (AxisValue :type Float%20%28single-precision%29))
  (Pawn|Input|AddMovementInput (Transformation|GetActorRightVector) AxisValue false))

(fn ConstructionScript)

(fn UpdatePlayerAim
  (bind _returnvalue (Game|GetPlayerCharacter 0))
  (bind _returnvalue_2 (Transformation|GetActorRotation _returnvalue))
  (Pawn|SetControlRotation (Game|GetPlayerController 0) (Math|Rotator|MakeRotator (.roll _returnvalue_2) (.pitch _returnvalue_2) (+ (* (Input|AxisValues|GetControllerAimRight/Left) (* (Variables|Default|GetRotationSpeed) (Utilities|Time|GetWorldDeltaSeconds))) (.yaw _returnvalue_2)))))